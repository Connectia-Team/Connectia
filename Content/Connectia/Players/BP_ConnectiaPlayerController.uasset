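; BP_ConnectiaPlayerController is the player controller for Connectia, linking the player to the in-game HUD and handling the death screen.
; On BeginPlay it retries each tick until the HUD is valid, then caches it as HUD_InGame.
; Die waits briefly, switches input to UI only and plays the HUD widget's fade to black.
; The 8 key adds XP through the player state, apparently as a debug shortcut.
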(event Custom|Die
  (Utilities|FlowControl|Delay 1.0)
  (Input|SetInputModeUIOnly self 0 "DoNotLock" false)
  (Default|FadeinBlackness (Variables|/Game/Connectia/UI/HUD_InGame.HUD_InGame_C|GetWidget (Variables|Default|GetInGameHUD)) "Forward" 1.0))

(event EventBeginPlay
  (bind _returnvalue (HUD|GetHUD))
  (Utilities|IsValid _returnvalue :!label _label
    (:Is%20Valid
      (bind _ashud_in_game (Utilities|Casting|CastToHUD_InGame _returnvalue))
      (Variables|Default|SetInGameHUD _ashud_in_game))
    (:Is%20Not%20Valid
      (Utilities|FlowControl|DelayUntilNextTick)
      (goto _label))))

(event Input|KeyboardEvents|8
  (params (Key :type Key%20Structure :default "None"))
  (:Pressed
    (bind _asbp_connectia_player_state (Utilities|Casting|CastToBP_ConnectiaPlayerState (Game|GetPlayerState 0)))
    (Default|AddXP _asbp_connectia_player_state 0.7)))

(fn ConstructionScript)