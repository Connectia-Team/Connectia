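; Connectia player state that holds the player's team and XP/level progression.
; The server picks a random team from the game mode at BeginPlay, and OnRep_Team notifies the character.
; BeginPlay also creates the XP widget, which AddXP and IncreaseLevel update.
; Overflow XP carries recursively into the next level up to level 10, with a rising threshold and a timeline intended to smooth the bar.
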(event EventBeginPlay
  (Utilities|FlowControl|Sequence
    (:then_0
      (Networking|SwitchHasAuthority
        (:Authority
          (bind _asbp_connectia_test_game_mode (Utilities|Casting|CastToBP_ConnectiaTestGameMode (Game|GetGameMode)))
          (Variables|Default|SetTeam (.OutItem (Utilities|Array|Random (Variables|/Game/Connectia/GameModes/BP_ConnectiaTestGameMode.BP_ConnectiaTestGameMode_C|GetTeams _asbp_connectia_test_game_mode)))))))
    (:then_1
      (bind _returnvalue (UserInterface|CreateWidget "/Game/Connectia/UI/WBP_XP.WBP_XP_C"))
      (Variables|Default|SetPlayerWidgetReference _returnvalue)
      (UserInterface|Viewport|AddtoViewport (Variables|Default|GetPlayerWidgetReference) 0))))

(fn ConstructionScript)

(fn OnRepTeam
  (bind _asbp_connectia_character (Utilities|Casting|CastToBP_ConnectiaCharacter (PlayerState|GetPawn)))
  (Default|TeamChanged _asbp_connectia_character))

(fn AddXP
  (params (Amount :type Float%20%28double-precision%29))
  (LocalVariables|SetlocalAddedXP (+ (Variables|Default|GetCurrentXP) Amount))
  (Variables|Default|SetOldXP (/ (Variables|Default|GetCurrentXP) (Variables|Default|GetMaxXP)))
  (if (!= (Variables|Default|GetCurrentLevel) 10)
    (if (> (LocalVariables|GetlocalAddedXP) (Variables|Default|GetMaxXP))
      (LocalVariables|SetlocalGivenXP (- (Variables|Default|GetMaxXP) (Variables|Default|GetCurrentXP)))
      (LocalVariables|SetlocalExtraXP (- (LocalVariables|GetlocalAddedXP) (Variables|Default|GetMaxXP)))
      (Variables|Default|SetCurrentXP (+ (Variables|Default|GetCurrentXP) (LocalVariables|GetlocalGivenXP)))
      (else
        (Variables|Default|SetCurrentXP (LocalVariables|GetlocalAddedXP))))
    (Development|PrintString (Utilities|String|ToString(Text) (Utilities|Text|FormatText "{Current}/{Max}" (* (Variables|Default|GetCurrentXP) 1e+02) (* (Variables|Default|GetMaxXP) 1e+02))))
    (Default|UpdateXP (Variables|Default|GetPlayerWidgetReference))
    (Components|Timeline|PlayfromStart (Variables|Default|GetXPSmooth))
    (LocalVariables|SetlocalGivenXP 0.0)
    (CallFunction|IncreaseLevel (LocalVariables|GetlocalExtraXP))))

(fn IncreaseLevel
  (params (ExtraXP :type Float%20%28double-precision%29))
  (bind _playerwidgetreference (Variables|Default|GetPlayerWidgetReference))
  (if (>= (Variables|Default|GetCurrentXP) (Variables|Default|GetMaxXP))
    (Variables|Default|SetCurrentLevel (+ (Variables|Default|GetCurrentLevel) 1))
    (Variables|Default|SetCurrentXP 0.0)
    (Variables|Default|SetMaxXP (Math|Float|Clamp(Float) (+ (Variables|Default|GetMaxXP) 0.5) 0.0 1e+03))
    (Default|UpdateLevel _playerwidgetreference)
    (Default|UpdateXP _playerwidgetreference)
    (if (> ExtraXP 0.0)
      (CallFunction|AddXP ExtraXP))))

(fn GetXP
  (return (Variables|Default|GetCurrentXP) (Variables|Default|GetMaxXP)))

(fn GetLvl
  (return (Variables|Default|GetCurrentLevel)))