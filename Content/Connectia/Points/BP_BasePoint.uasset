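; Base capture point that teams take over, capturable by a team only if that team holds an adjacent point.
; Start and stop calls write a single CaptureState struct, and the authority's Tick advances its progress until the recapturing team becomes owner and OnCaptured fires.
; The struct's RepNotify pushes state to child actors implementing BPI_Indicator, which the construction script caches and initializes.
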(event EventTick
  (params (DeltaSeconds :type Float%20%28single-precision%29))
  (Networking|SwitchHasAuthority
    (:Authority
      (if (CallFunction|IsBeingCaptured)
        (CallFunction|IncreaseCaptureProgress (* (Variables|Default|GetCaptureSpeedPerSecond) (Utilities|Time|GetWorldDeltaSeconds)))))))

(fn ConstructionScript
  (CallFunction|CacheChildIndicators)
  (CallFunction|UpdateIndicators))

(fn GetIndicators
  (return (Variables|Default|GetCachedChildIndicators)))

(fn CacheChildIndicators
  (Utilities|Array|Clear (Variables|Default|GetCachedChildIndicators))
  (for _array_element (Actor|GetAllChildActors true)
    (bind _asbpi_indicator (Utilities|Casting|CastToBPI_Indicator _array_element))
    (Utilities|Array|Add (Variables|Default|GetCachedChildIndicators) _asbpi_indicator)))

(fn UpdateIndicators
  (for _array_element (CallFunction|GetIndicators)
    (Default|Update _array_element (Variables|Default|GetCaptureState))))

(fn StartCapture
  (params (Team :type PDA%20Team%20Object%20Reference))
  (Variables|Default|SetCaptureState (Utilities|Struct|MakeS_CaptureState (CallFunction|GetCurrentTeam) Team 0.0 true)))

(fn StopCapture
  (Variables|Default|SetCaptureState (Utilities|Struct|MakeS_CaptureState (CallFunction|GetCurrentTeam) "/Game/Connectia/Teams/Team_None.Team_None" 0.0 false)))

(fn IncreaseCaptureProgress
  (params (DeltaProgress :type Float%20%28double-precision%29))
  (bind _output_get (LocalVariables|SetNewProgress (+ DeltaProgress (CallFunction|GetRecapturingProgress))))
  (if (>= _output_get 1.0)
    (Variables|Default|SetCaptureState (Utilities|Struct|MakeS_CaptureState (CallFunction|GetRecapturingTeam) "/Game/Connectia/Teams/Team_None.Team_None" 0.0 false))
    (Default|CallOnCaptured self)
    (else
      (Variables|Default|SetCaptureState (Utilities|Struct|MakeS_CaptureState (CallFunction|GetCurrentTeam) (CallFunction|GetRecapturingTeam) (LocalVariables|GetNewProgress) true)))))

(fn OnRepCaptureState
  (CallFunction|UpdateIndicators))

(fn GetCurrentTeam
  (return (.currentteam (Variables|Default|GetCaptureState))))

(fn GetRecapturingTeam
  (return (.recapturingteam (Variables|Default|GetCaptureState))))

(fn GetRecapturingProgress
  (return (.recapturingprogress (Variables|Default|GetCaptureState))))

(fn IsBeingCaptured
  (return (.isbeingcaptured (Variables|Default|GetCaptureState))))

(fn CanbeCapturedbyTeam
  (params (Team :type PDA%20Team%20Object%20Reference))
  (for _array_element (Variables|Default|GetAdjacentPointsTransient)
    (if (== (CallFunction|GetCurrentTeam _array_element) Team)
      (return true)))
  (return false))