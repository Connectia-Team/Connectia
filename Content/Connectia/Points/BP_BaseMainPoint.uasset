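; Base main point actor that owns a set of child PlayerStart actors and exposes them as spawn locations.
; The construction script runs the parent's logic, then rebuilds a cached list by filtering all descendant child actors for PlayerStarts.
; GetPlayerStarts returns that cached list, so callers avoid searching the child actors again.
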(fn ConstructionScript
  (|CallParentFunction)
  (CallFunction|CacheChildPlayerStarts))

(fn GetPlayerStarts
  (return (Variables|Default|GetCachedChildPlayerStarts)))

(fn CacheChildPlayerStarts
  (Utilities|Array|Clear (Variables|Default|GetCachedChildPlayerStarts))
  (for _array_element (Actor|GetAllChildActors true)
    (bind _asplayer_start (Utilities|Casting|CastToPlayerStart _array_element))
    (Utilities|Array|Add (Variables|Default|GetCachedChildPlayerStarts) _asplayer_start)))