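; BP_PointsManagerComponent is a component that acts as a registry of the level's points and wires.
; On BeginPlay it gathers all BP_BasePoint and BP_Wire actors and filters out the BP_BaseMainPoint ones.
; It maps each team to its main point, printing a red error when a team already has one.
; Getters expose all points, main points, wires and a team's main point.
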(event EventBeginPlay
  (Utilities|FlowControl|Sequence
    (:then_0
      (bind _outactors (Actor|GetAllActorsOfClass "/Game/Connectia/Points/BP_BasePoint.BP_BasePoint_C"))
      (Variables|Default|SetPoints _outactors))
    (:then_1
      (for _array_element (Variables|Default|GetPoints)
        (bind _asbp_base_main_point (Utilities|Casting|CastToBP_BaseMainPoint _array_element))
        (Utilities|Array|Add (Variables|Default|GetMainPoints) _asbp_base_main_point)))
    (:then_2
      (for _array_element_2 (Variables|Default|GetMainPoints)
        (if (Utilities|Map|Contains (Variables|Default|GetTeamToMainPointMap) (Default|GetCurrentTeam _array_element_2))
          (Development|PrintString "More than two main points of the same team" true true "(R=1.000000,G=0.000000,B=0.000000,A=1.000000)")
          (else
            (Utilities|Map|Add (Variables|Default|GetTeamToMainPointMap) (Default|GetCurrentTeam _array_element_2) _array_element_2)))))
    (:then_3
      (bind _outactors_2 (Actor|GetAllActorsOfClass "/Game/Connectia/Points/Connections/BP_Wire.BP_Wire_C"))
      (Variables|Default|SetWires _outactors_2))))

(fn GetAllPoints
  (return (Variables|Default|GetPoints)))

(fn GetMainPoints
  (return (Variables|Default|GetMainPoints)))

(fn GetAllWires
  (return (Variables|Default|GetWires)))

(fn GetTeamMainPoint
  (params (Team :type PDA%20Team%20Object%20Reference%20%28by%20ref%29))
  (return (.Value (Utilities|Map|Find (Variables|Default|GetTeamToMainPointMap) Team))))