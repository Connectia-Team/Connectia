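; BP_FlagIndicator is a capture-point flag indicator that shows team ownership and recapture progress.
; The construction script makes the mesh's second material slot a dynamic instance, which is cached on BeginPlay.
; Its Update event takes a capture state and feeds the new team color, previous team color and recapture progress into material parameters, leaving the color transition to the material.
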(event EventUpdate
  (params (NewCaptureState :type S%20Capture%20State%20Structure))
  (Rendering|Material|SetVectorParameterValue (Variables|Default|GetMaterial) "NewColor" (Variables|/Game/Connectia/Teams/PDA_Team.PDA_Team_C|GetColor (.newteam NewCaptureState)) :!class /Script/Engine.MaterialInstanceDynamic)
  (Rendering|Material|SetVectorParameterValue (Variables|Default|GetMaterial) "PreviousColor" (Variables|/Game/Connectia/Teams/PDA_Team.PDA_Team_C|GetColor (.previousteam NewCaptureState)) :!class /Script/Engine.MaterialInstanceDynamic)
  (Rendering|Material|SetScalarParameterValue (Variables|Default|GetMaterial) "NewColorProgress" (.recaptureprogress NewCaptureState) :!class /Script/Engine.MaterialInstanceDynamic))

(event EventBeginPlay
  (bind _asmaterial_instance_dynamic (Utilities|Casting|CastToMaterialInstanceDynamic (Rendering|Material|GetMaterial (Variables|Default|GetMesh) 1)))
  (Variables|Default|SetMaterial _asmaterial_instance_dynamic))

(fn ConstructionScript
  (CallFunction|MakeMeshMaterialDynamic (Variables|Default|GetMesh) 1))