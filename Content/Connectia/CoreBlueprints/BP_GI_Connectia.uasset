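; BP_GI_Connectia is the Connectia Game Instance Blueprint, which handles session cleanup on shutdown and on network or travel failures.
; Shutdown, network error and travel error events each print a debug message, with the failure type and, for network errors, the server flag.
; All three then converge on one DestroySession call for player controller 0.
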(event EventShutdown
  (Development|PrintString "GAME INSTANCE SHUTDOWN")
  (|DestroySession (Game|GetPlayerController 0)))

(event EventHandleNetworkError
  (params (FailureType :type ENetworkFailure%20Enum :default "NetDriverAlreadyExists") (bIsServer :type Boolean))
  (Development|PrintText (Utilities|Text|FormatText "NetworkError. FailureType={FailureType}, IsServer={IsServer}" (Utilities|String|EnumtoString FailureType) bIsServer))
  (|DestroySession (Game|GetPlayerController 0)))

(event EventHandleTravelError
  (params (FailureType :type ETravelFailure%20Enum :default "NoLevel"))
  (Development|PrintText (Utilities|Text|FormatText "TravelError. FailureType={FailureType}" (Utilities|String|EnumtoString FailureType)))
  (|DestroySession (Game|GetPlayerController 0)))