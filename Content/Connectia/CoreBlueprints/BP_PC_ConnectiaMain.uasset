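; Player controller for Connectia that turns input into stat upgrades and UI toggles.
; Five Boost Stat actions each call BoostStat on the player state's LevelingComponent for Damage, Range, FireRate, Stability or MaxCap.
; Another action fires the OnSwitchShowPlayerStats dispatcher, and a debug key grants XP only with authority.
; A helper function returns the player widget cast to WBP_PlayerMain.
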(event Input|ActionEvents|InputActionBoostStat4
  (params (Key :type Key%20Structure :default "None"))
  (:Pressed
    (bind _asbp_ps_connectia_main (Utilities|Casting|CastToBP_PS_ConnectiaMain (Variables|Default|GetPlayerState)))
    (Default|BoostStat (Variables|/Game/Connectia/CoreBlueprints/BP_PS_ConnectiaMain.BP_PS_ConnectiaMain_C|GetLevelingComponent _asbp_ps_connectia_main) "Stability")))

(event Input|ActionEvents|InputActionBoostStat5
  (params (Key :type Key%20Structure :default "None"))
  (:Pressed
    (bind _asbp_ps_connectia_main (Utilities|Casting|CastToBP_PS_ConnectiaMain (Variables|Default|GetPlayerState)))
    (Default|BoostStat (Variables|/Game/Connectia/CoreBlueprints/BP_PS_ConnectiaMain.BP_PS_ConnectiaMain_C|GetLevelingComponent _asbp_ps_connectia_main) "MaxCap")))

(event Input|ActionEvents|InputActionBoostStat1
  (params (Key :type Key%20Structure :default "None"))
  (:Pressed
    (bind _asbp_ps_connectia_main (Utilities|Casting|CastToBP_PS_ConnectiaMain (Variables|Default|GetPlayerState)))
    (Default|BoostStat (Variables|/Game/Connectia/CoreBlueprints/BP_PS_ConnectiaMain.BP_PS_ConnectiaMain_C|GetLevelingComponent _asbp_ps_connectia_main) "Damage")))

(event Input|ActionEvents|InputActionBoostStat2
  (params (Key :type Key%20Structure :default "None"))
  (:Pressed
    (bind _asbp_ps_connectia_main (Utilities|Casting|CastToBP_PS_ConnectiaMain (Variables|Default|GetPlayerState)))
    (Default|BoostStat (Variables|/Game/Connectia/CoreBlueprints/BP_PS_ConnectiaMain.BP_PS_ConnectiaMain_C|GetLevelingComponent _asbp_ps_connectia_main) "Range")))

(event Input|ActionEvents|InputActionBoostStat3
  (params (Key :type Key%20Structure :default "None"))
  (:Pressed
    (bind _asbp_ps_connectia_main (Utilities|Casting|CastToBP_PS_ConnectiaMain (Variables|Default|GetPlayerState)))
    (Default|BoostStat (Variables|/Game/Connectia/CoreBlueprints/BP_PS_ConnectiaMain.BP_PS_ConnectiaMain_C|GetLevelingComponent _asbp_ps_connectia_main) "FireRate")))

(event Input|ActionEvents|InputActionSwitchShowPlayerStats
  (params (Key :type Key%20Structure :default "None"))
  (:Pressed
    (Default|CallOnSwitchShowPlayerStats self)))

(event Input|KeyboardEvents|DebugKey0
  (params (Key :type Key%20Structure :default "None") (ActionValue :type Input%20Action%20Value%20Structure))
  (:Pressed
    (Networking|SwitchHasAuthority
      (:Authority
        (bind _asbp_ps_connectia_main (Utilities|Casting|CastToBP_PS_ConnectiaMain (Variables|Default|GetPlayerState)))
        (Default|AddXP (Variables|/Game/Connectia/CoreBlueprints/BP_PS_ConnectiaMain.BP_PS_ConnectiaMain_C|GetLevelingComponent _asbp_ps_connectia_main) 1.5)))))

(fn ConstructionScript)

(fn GetPlayerMainWidget
  (bind _aswbp_player_main (Utilities|Casting|CastToWBP_PlayerMain (Variables|Default|GetPlayerWidget))) ; static_cast
  (return _aswbp_player_main))