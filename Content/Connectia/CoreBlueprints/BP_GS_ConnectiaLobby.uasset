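; BP_GS_ConnectiaLobby is the lobby Game State for Connectia, holding replicated match-start and vote status.
; It tracks whether the match is starting, the starting countdown, the voted count and the needed count.
; Each variable's RepNotify calls the same OnStatusUpdated dispatcher, so listeners get one notification for any status change.
; The file contains no logic that sets these values.
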(fn ConstructionScript)

(fn OnRepIsMatchStarting
  (Default|CallOnStatusUpdated self))

(fn OnRepMatchStartingCountdown
  (Default|CallOnStatusUpdated self))

(fn OnRepVotedCount
  (Default|CallOnStatusUpdated self))

(fn OnRepNeedCount
  (Default|CallOnStatusUpdated self))