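; Player controller for the Connectia lobby that lets a player vote or unvote for starting the match.
; On BeginPlay it adds the lobby status widget for the local controller and sets a flag that, with the parent's check, determines IsInitialized.
; Both vote inputs feed VoteForMatch, which stores the Voted state and notifies the lobby game mode that votes changed.
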(event Custom|VoteForMatch
  (params (Positive :type Boolean))
  (Variables|Default|SetVoted Positive)
  (bind _asbp_gm_connectia_lobby (Utilities|Casting|CastToBP_GM_ConnectiaLobby (Game|GetGameMode)))
  (Default|VotesUpdated _asbp_gm_connectia_lobby))

(event EventBeginPlay
  (|CallParentFunction)
  (Utilities|FlowControl|Sequence
    (:then_0
      (if (Pawn|IsLocalPlayerController)
        (bind _returnvalue (UserInterface|CreateWidget "/Game/Connectia/UI/WBP_LobbyStatus.WBP_LobbyStatus_C" self))
        (UserInterface|Viewport|AddtoViewport _returnvalue 0)))
    (:then_1
      (Variables|Default|SetIsInitializedVar_Lobby true))))

(event Input|ActionEvents|InputActionVoteForMatchStart
  (params (Key :type Key%20Structure :default "None"))
  (:Pressed
    (Variables|Default|SetVoted true)
    (CallFunction|VoteforMatch (Variables|Default|GetVoted))))

(event Input|ActionEvents|InputActionUnvoteForMatchStart
  (params (Key :type Key%20Structure :default "None"))
  (:Pressed
    (Variables|Default|SetVoted false)
    (CallFunction|VoteforMatch (Variables|Default|GetVoted))))

(fn ConstructionScript
  (|CallParentFunction))

(fn IsInitialized
  (bind _isinitialized (|CallParentFunction))
  (return (and _isinitialized (Variables|Default|GetIsInitializedVar_Lobby))))