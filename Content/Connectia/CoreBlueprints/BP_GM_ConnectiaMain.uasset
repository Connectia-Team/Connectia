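; Main Connectia game mode that balances players across teams and spawns their characters.
; On login or controller swap, it counts team sizes in the GameState's TeamsMap and picks randomly among the teams gathered as smallest.
; Team changes update both that map and the PlayerState's Team, with logout removing the player and resetting it to unassigned.
; Starting players possess a new BP_ConnectiaCharacter spawned at a random team start matching their team's tag.
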(event EventPostLogin
  (params (NewPlayer :type Player%20Controller%20Object%20Reference))
  (bind _asbp_pc_connectia_main (Utilities|Casting|CastToBP_PC_ConnectiaMain NewPlayer))
  (CallFunction|ProcessNewPC _asbp_pc_connectia_main))

(event EventOnSwapPlayerControllers
  (params (OldPC :type Player%20Controller%20Object%20Reference) (NewPC :type Player%20Controller%20Object%20Reference))
  (bind _asbp_pc_connectia_main (Utilities|Casting|CastToBP_PC_ConnectiaMain NewPC))
  (CallFunction|ProcessNewPC _asbp_pc_connectia_main))

(event EventOnLogout
  (params (ExitingController :type Controller%20Object%20Reference))
  (bind _asbp_pc_connectia_main (Utilities|Casting|CastToBP_PC_ConnectiaMain ExitingController))
  (CallFunction|ProcessLeftPC _asbp_pc_connectia_main))

(event EventHandleStartingNewPlayer
  (params (NewPlayer :type Player%20Controller%20Object%20Reference))
  (bind _asbp_pc_connectia_main (Utilities|Casting|CastToBP_PC_ConnectiaMain NewPlayer))
  (CallFunction|SpawnPC _asbp_pc_connectia_main))

(fn ConstructionScript)

(fn ProcessNewPC
  (params (NewPC :type BP%20PC%20Connectia%20Main%20Object%20Reference))
  (CallFunction|AssignNewPCATeam NewPC))

(fn ProcessLeftPC
  (params (LeftPC :type BP%20PC%20Connectia%20Main%20Object%20Reference))
  (bind _asbp_ps_connectia_main (Utilities|Casting|CastToBP_PS_ConnectiaMain (Variables|/Script/Engine.Controller|GetPlayerState LeftPC)))
  (CallFunction|RemovePSfromTeam _asbp_ps_connectia_main))

(fn AssignNewPCATeam
  (params (PC :type BP%20PC%20Connectia%20Main%20Object%20Reference))
  (bind _asbp_gs_connectia_main (Utilities|Casting|CastToBP_GS_ConnectiaMain (Game|GetGameState)))
  (for (_array_element _array_index) (Variables|Default|GetAllTeams)
    (Utilities|Array|SetArrayElem (LocalVariables|GetTeamsSizes) _array_index (Utilities|Array|Length (.psarray (.Value (Utilities|Map|Find (Variables|/Game/Connectia/CoreBlueprints/BP_GS_ConnectiaMain.BP_GS_ConnectiaMain_C|GetTeamsMap _asbp_gs_connectia_main) _array_element)))) true))
  (LocalVariables|SetMinTeamSize (.MinValue (Math|Integer|MinOfIntArray (LocalVariables|GetTeamsSizes))))
  (for (_array_element_2 _array_index_2) (Variables|Default|GetAllTeams)
    (if (== (Utilities|Array|Get(acopy) (LocalVariables|GetTeamsSizes) _array_index_2) (LocalVariables|GetMinTeamSize))
      (Utilities|Array|Add (LocalVariables|GetMinTeams) _array_element_2)))
  (bind _asbp_ps_connectia_main (Utilities|Casting|CastToBP_PS_ConnectiaMain (Variables|/Script/Engine.Controller|GetPlayerState PC)))
  (CallFunction|AddPStoTeam _asbp_ps_connectia_main (.OutItem (Utilities|Array|Random (LocalVariables|GetMinTeams)))))

(fn AddPStoTeam
  (params (PS :type BP%20PS%20Connectia%20Main%20Object%20Reference) (Team :type PDA%20Team%20Object%20Reference))
  (bind _asbp_gs_connectia_main (Utilities|Casting|CastToBP_GS_ConnectiaMain (Game|GetGameState)))
  (bind _output_get (LocalVariables|SetPS%20Array%20Buf (.psarray (.Value (Utilities|Map|Find (Variables|/Game/Connectia/CoreBlueprints/BP_GS_ConnectiaMain.BP_GS_ConnectiaMain_C|GetTeamsMap _asbp_gs_connectia_main) Team)))))
  (Utilities|Array|Add _output_get PS)
  (Utilities|Map|Add (Variables|/Game/Connectia/CoreBlueprints/BP_GS_ConnectiaMain.BP_GS_ConnectiaMain_C|GetTeamsMap _asbp_gs_connectia_main) Team (Utilities|Struct|MakeS_PSConnectiaMainArray _output_get))
  (Variables|/Game/Connectia/CoreBlueprints/BP_PS_ConnectiaMain.BP_PS_ConnectiaMain_C|SetTeam PS Team)
  (Development|PrintText (Utilities|Text|FormatText "{PS} added to {Team} team" PS (Variables|/Game/Connectia/Teams/PDA_Team.PDA_Team_C|GetShortName Team))))

(fn RemovePSfromTeam
  (params (PS :type BP%20PS%20Connectia%20Main%20Object%20Reference))
  (bind _asbp_gs_connectia_main (Utilities|Casting|CastToBP_GS_ConnectiaMain (Game|GetGameState)))
  (bind _output_get (LocalVariables|SetPS%20Array%20Buf (.psarray (.Value (Utilities|Map|Find (Variables|/Game/Connectia/CoreBlueprints/BP_GS_ConnectiaMain.BP_GS_ConnectiaMain_C|GetTeamsMap _asbp_gs_connectia_main) (Variables|/Game/Connectia/CoreBlueprints/BP_PS_ConnectiaMain.BP_PS_ConnectiaMain_C|GetTeam PS))))))
  (if (.ReturnValue (Utilities|Map|Find (Variables|/Game/Connectia/CoreBlueprints/BP_GS_ConnectiaMain.BP_GS_ConnectiaMain_C|GetTeamsMap _asbp_gs_connectia_main) (Variables|/Game/Connectia/CoreBlueprints/BP_PS_ConnectiaMain.BP_PS_ConnectiaMain_C|GetTeam PS)))
    (Utilities|Array|RemoveItem _output_get PS)
    (Utilities|Map|Add (Variables|/Game/Connectia/CoreBlueprints/BP_GS_ConnectiaMain.BP_GS_ConnectiaMain_C|GetTeamsMap _asbp_gs_connectia_main) (Variables|/Game/Connectia/CoreBlueprints/BP_PS_ConnectiaMain.BP_PS_ConnectiaMain_C|GetTeam PS) (Utilities|Struct|MakeS_PSConnectiaMainArray _output_get)))
  (Development|PrintText (Utilities|Text|FormatText "{PS} removed from {Team} team" PS (Variables|/Game/Connectia/Teams/PDA_Team.PDA_Team_C|GetShortName (Variables|/Game/Connectia/CoreBlueprints/BP_PS_ConnectiaMain.BP_PS_ConnectiaMain_C|GetTeam PS))))
  (Variables|/Game/Connectia/CoreBlueprints/BP_PS_ConnectiaMain.BP_PS_ConnectiaMain_C|SetTeam PS "/Game/Connectia/Teams/Team_Unassigned.Team_Unassigned"))

(fn SpawnPC
  (params (PC :type BP%20PC%20Connectia%20Main%20Object%20Reference))
  (bind _asbp_ps_connectia_main (Utilities|Casting|CastToBP_PS_ConnectiaMain (Variables|/Script/Engine.Controller|GetPlayerState PC)))
  (bind _outactors (Actor|GetAllActorsOfClasswithTag "/Game/Connectia/CoreBlueprints/BP_ConnectiaTeamPlayerStart.BP_ConnectiaTeamPlayerStart_C" (Variables|/Game/Connectia/Teams/PDA_Team.PDA_Team_C|GetTagName (Variables|/Game/Connectia/CoreBlueprints/BP_PS_ConnectiaMain.BP_PS_ConnectiaMain_C|GetTeam _asbp_ps_connectia_main))))
  (if (Utilities|Array|IsNotEmpty _outactors)
    (bind _returnvalue (Game|SpawnActorfromClass "/Game/Connectia/Characters/BP_ConnectiaCharacter.BP_ConnectiaCharacter_C" (Transformation|GetActorTransform (.OutItem (Utilities|Array|Random _outactors))) "Undefined" 0 0))
    (Pawn|Possess PC _returnvalue)))