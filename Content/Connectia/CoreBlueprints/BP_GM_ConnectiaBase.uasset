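; Base game mode for Connectia that handles spawning and respawning of player pawns.
; It overrides default pawn spawning to return nothing, and instead calls RespawnPC when a new Connectia player controller starts.
; RespawnPC uses TrySpawnPC to spawn the default pawn at a random PlayerStart and possess it.
; On success it calls ClientRespawn on the controller, flagging whether this is the first spawn.
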(event EventHandleStartingNewPlayer
  (params (NewPlayer :type Player%20Controller%20Object%20Reference))
  (bind _asbp_pc_connectia_base (Utilities|Casting|CastToBP_PC_ConnectiaBase NewPlayer))
  (CallFunction|RespawnPC _asbp_pc_connectia_base true))

(fn ConstructionScript)

(fn TrySpawnPC
  (params (PC :type BP%20PC%20Connectia%20Base%20Object%20Reference))
  (bind _outactors (Actor|GetAllActorsOfClass "/Script/Engine.PlayerStart"))
  (if (Utilities|Array|IsNotEmpty _outactors)
    (bind _returnvalue (Game|SpawnActorfromClass (Variables|Default|GetDefaultPawnClass) (Transformation|GetActorTransform (.OutItem (Utilities|Array|Random _outactors))) "Undefined" 0 0))
    (Pawn|Possess PC _returnvalue)
    (return true)
    (else
      (return false))))

(fn RespawnPC
  (params (PC :type BP%20PC%20Connectia%20Base%20Object%20Reference) (IsFirstRespawn :type Boolean))
  (bind _success (CallFunction|TrySpawnPC PC))
  (if _success
    (Default|ClientRespawn PC IsFirstRespawn)))

(fn SpawnDefaultPawnfor
  (params (NewPlayer :type Controller%20Object%20Reference) (StartSpot :type Actor%20Object%20Reference))
  (return 0))