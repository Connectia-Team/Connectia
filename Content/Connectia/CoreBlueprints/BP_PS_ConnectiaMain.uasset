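; Player state for Connectia that tracks a player's team, XP and level, with a replicated team change notifying the possessed character.
; AddXP stops gaining at level 10, fills the bar up to MaxXP and passes overflow to IncreaseLevel, which raises the threshold and recursively re-adds the remainder.
; It updates the player widget directly and plays a timeline meant to smooth the XP bar, marked to move into the widget.
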(fn ConstructionScript)

(fn OnRepTeam
  (bind _asbp_connectia_character (Utilities|Casting|CastToBP_ConnectiaCharacter (PlayerState|GetPawn)))
  (Default|TeamChanged _asbp_connectia_character))

(fn AddXP
  (params (Amount :type Float%20%28double-precision%29))
  (LocalVariables|SetlocalAddedXP (+ (Variables|Default|GetCurrentXP) Amount))
  (Variables|Default|SetOldXP (/ (Variables|Default|GetCurrentXP) (Variables|Default|GetMaxXP)))
  (if (!= (Variables|Default|GetCurrentLevel) 10)
    (if (> (LocalVariables|GetlocalAddedXP) (Variables|Default|GetMaxXP))
      (LocalVariables|SetlocalGivenXP (- (Variables|Default|GetMaxXP) (Variables|Default|GetCurrentXP)))
      (LocalVariables|SetlocalExtraXP (- (LocalVariables|GetlocalAddedXP) (Variables|Default|GetMaxXP)))
      (Variables|Default|SetCurrentXP (+ (Variables|Default|GetCurrentXP) (LocalVariables|GetlocalGivenXP)))
      (else
        (Variables|Default|SetCurrentXP (LocalVariables|GetlocalAddedXP))))
    (Development|PrintString (Utilities|String|ToString(Text) (Utilities|Text|FormatText "{Current}/{Max}" (* (Variables|Default|GetCurrentXP) 1e+02) (* (Variables|Default|GetMaxXP) 1e+02))))
    (Utilities|IsValid (Variables|Default|GetPlayerWidgetReference)
      (:Is%20Valid
        (Default|UpdateXP (Variables|Default|GetPlayerWidgetReference))
        (Components|Timeline|PlayfromStart (Variables|Default|GetXPSmooth))
        (LocalVariables|SetlocalGivenXP 0.0)
        (CallFunction|IncreaseLevel (LocalVariables|GetlocalExtraXP)))
      (:Is%20Not%20Valid
        (bind _asbp_pc_connectia_base (Utilities|Casting|CastToBP_PC_ConnectiaBase (Game|GetPlayerController 0)))
        (bind _asbp_hud_in_game (Utilities|Casting|CastTo (HUD|GetHUD _asbp_pc_connectia_base)))
        (Variables|Default|SetPlayerWidgetReference _asbp_hud_in_game 0)))))

(fn IncreaseLevel
  (params (ExtraXP :type Float%20%28double-precision%29))
  (bind _playerwidgetreference (Variables|Default|GetPlayerWidgetReference))
  (if (>= (Variables|Default|GetCurrentXP) (Variables|Default|GetMaxXP))
    (Variables|Default|SetCurrentLevel (+ (Variables|Default|GetCurrentLevel) 1))
    (Variables|Default|SetCurrentXP 0.0)
    (Variables|Default|SetMaxXP (Math|Float|Clamp(Float) (+ (Variables|Default|GetMaxXP) 0.5) 0.0 1e+03))
    (Utilities|IsValid _playerwidgetreference
      (:Is%20Valid
        (Default|UpdateLevel _playerwidgetreference)
        (Default|UpdateXP _playerwidgetreference)
        (if (> ExtraXP 0.0)
          (CallFunction|AddXP ExtraXP)))
      (:Is%20Not%20Valid
        (bind _asbp_pc_connectia_base (Utilities|Casting|CastToBP_PC_ConnectiaBase (Game|GetPlayerController 0)))
        (Utilities|Casting|CastTo (HUD|GetHUD _asbp_pc_connectia_base))))))

(fn GetXP
  (return (Variables|Default|GetCurrentXP) (Variables|Default|GetMaxXP)))

(fn GetLvl
  (return (Variables|Default|GetCurrentLevel)))