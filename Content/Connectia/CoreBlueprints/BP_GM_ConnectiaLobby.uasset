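; Lobby game mode for Connectia that starts a match countdown once every player has voted.
; Player joins, leaves, controller swaps and VotesUpdated calls trigger a recount of each lobby controller's vote, written with the player count to BP_GS_ConnectiaLobby.
; When the counts match, a looping one-second timer decrements the game state's countdown.
; At zero it only clears the timer and prints a message, with no travel to a match.
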(event Custom|VotesUpdated
  (CallFunction|TrytoStartMatch))

(event Custom|StartMatchCountdown
  (bind _asbp_gs_connectia_lobby (Utilities|Casting|CastToBP_GS_ConnectiaLobby (Game|GetGameState)))
  (Variables|/Game/Connectia/CoreBlueprints/BP_GS_ConnectiaLobby.BP_GS_ConnectiaLobby_C|SetMatchStartingCountdown _asbp_gs_connectia_lobby (Variables|Default|GetTotalCountdownUntilMatchStart))
  (Variables|/Game/Connectia/CoreBlueprints/BP_GS_ConnectiaLobby.BP_GS_ConnectiaLobby_C|SetIsMatchStarting _asbp_gs_connectia_lobby true)
  (bind _returnvalue (Utilities|Time|SetTimerbyEvent (delegate Custom|OnCountdownTimer) 1.0 true)))

(event Custom|OnCountdownTimer
  (bind _output_get (Variables|/Game/Connectia/CoreBlueprints/BP_GS_ConnectiaLobby.BP_GS_ConnectiaLobby_C|SetMatchStartingCountdown (stale Custom|StartMatchCountdown _asbp_gs_connectia_lobby) (- (Variables|/Game/Connectia/CoreBlueprints/BP_GS_ConnectiaLobby.BP_GS_ConnectiaLobby_C|GetMatchStartingCountdown (stale Custom|StartMatchCountdown _asbp_gs_connectia_lobby)) 1)))
  (if (<= _output_get 0)
    (Utilities|Time|ClearandInvalidateTimerbyHandle (stale Custom|StartMatchCountdown _returnvalue))
    (Development|PrintString "Starting match")))

(event EventPostLogin
  (params (NewPlayer :type Player%20Controller%20Object%20Reference))
  (CallFunction|VotesUpdated))

(event EventOnSwapPlayerControllers
  (params (OldPC :type Player%20Controller%20Object%20Reference) (NewPC :type Player%20Controller%20Object%20Reference))
  (CallFunction|VotesUpdated))

(event EventOnLogout
  (params (ExitingController :type Controller%20Object%20Reference))
  (CallFunction|VotesUpdated))

(fn ConstructionScript)

(fn TrytoStartMatch
  (bind _asbp_gs_connectia_lobby (Utilities|Casting|CastToBP_GS_ConnectiaLobby (Game|GetGameState)))
  (bind _output_get (Variables|/Game/Connectia/CoreBlueprints/BP_GS_ConnectiaLobby.BP_GS_ConnectiaLobby_C|SetNeedCount _asbp_gs_connectia_lobby (Utilities|Array|Length (Variables|/Script/Engine.GameStateBase|GetPlayerArray _asbp_gs_connectia_lobby))))
  (for _array_element (Variables|/Script/Engine.GameStateBase|GetPlayerArray _asbp_gs_connectia_lobby)
    (bind _asbp_pc_connectia_lobby (Utilities|Casting|CastToBP_PC_ConnectiaLobby (Game|GetPlayerController _array_element)))
    (|SetBy-RefVar (LocalVariables|GetVotedCount) (+ (LocalVariables|GetVotedCount) (Variables|/Game/Connectia/CoreBlueprints/BP_PC_ConnectiaLobby.BP_PC_ConnectiaLobby_C|GetVoted _asbp_pc_connectia_lobby))))
  (Variables|/Game/Connectia/CoreBlueprints/BP_GS_ConnectiaLobby.BP_GS_ConnectiaLobby_C|SetVotedCount _asbp_gs_connectia_lobby (LocalVariables|GetVotedCount))
  (if (== (LocalVariables|GetVotedCount) _output_get)
    (CallFunction|StartMatchCountdown)))