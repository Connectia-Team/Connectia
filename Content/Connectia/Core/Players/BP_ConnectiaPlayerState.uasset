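; Player state for Connectia that assigns each player a team and notifies their character when it changes.
; On BeginPlay, the authority picks a random entry from the test game mode's Teams array and stores it as the replicated Team.
; The Team RepNotify casts the owning pawn to the Connectia character and calls TeamChanged on it.
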(event EventBeginPlay
  (Utilities|FlowControl|Sequence
    (:then_0
      (Networking|SwitchHasAuthority
        (:Authority
          (bind _asbp_connectia_test_game_mode (Utilities|Casting|CastToBP_ConnectiaTestGameMode (Game|GetGameMode)))
          (Variables|Default|SetTeam (.OutItem (Utilities|Array|Random (Variables|/Game/Connectia/Core/GameModes/BP_ConnectiaTestGameMode.BP_ConnectiaTestGameMode_C|GetTeams _asbp_connectia_test_game_mode)))))))))

(fn ConstructionScript)

(fn OnRepTeam
  (bind _asbp_connectia_character (Utilities|Casting|CastToBP_ConnectiaCharacter (PlayerState|GetPawn)))
  (Default|TeamChanged _asbp_connectia_character))