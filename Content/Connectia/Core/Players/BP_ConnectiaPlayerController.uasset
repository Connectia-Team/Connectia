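; BP_ConnectiaPlayerController is the Connectia player controller, handling possession hotkeys and the player death screen.
; F unpossesses the current pawn, and G possesses the BP_ConnectiaCharacter returned by GetActorOfClass.
; The Die event switches input to UI only without locking the mouse, then casts the HUD to BP_HUD and plays its widget's fade to black.
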(event Custom|Die
  (Input|SetInputModeUIOnly self 0 "DoNotLock")
  (bind _asbp_hud (Utilities|Casting|CastToBP_HUD (HUD|GetHUD)))
  (Default|FadeinBlackness (Variables|/Game/Connectia/UI/BP_HUD.BP_HUD_C|GetHUD_WBP _asbp_hud) "Forward" 1.0))

(event Input|KeyboardEvents|F
  (params (Key :type Key%20Structure :default "None"))
  (:Pressed
    (Pawn|UnPossess)))

(event Input|KeyboardEvents|G
  (params (Key :type Key%20Structure :default "None"))
  (:Pressed
    (bind _returnvalue (Actor|GetActorOfClass "/Game/Connectia/Core/Characters/BP_ConnectiaCharacter.BP_ConnectiaCharacter_C"))
    (Pawn|Possess _returnvalue)))

(fn ConstructionScript)