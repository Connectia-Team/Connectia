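; Base weapon Blueprint for Connectia that mounts itself on the character that owns it.
; On BeginPlay it casts its owner to BP_ConnectiaCharacter, caches it, then attaches separate first-person and third-person meshes to sockets on the matching character meshes.
; The construction script converts materials on all its mesh components to dynamic instances.
; A note flags that owner caching ideally belongs in a C++ SetOwner override.
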(event EventBeginPlay
  (Utilities|FlowControl|Sequence
    (:then_0)
    (:then_1
      (CallFunction|CacheOwnerCharacter)
      (Utilities|IsValid (Variables|Default|GetCachedCharacter)
        (:Is%20Valid
          (CallFunction|AttachtoCachedCharacter))))))

(fn ConstructionScript
  (for _array_element (Actor|GetComponentsByClass "/Script/Engine.MeshComponent")
    (CallFunction|MakeMeshAllMaterialsDynamic _array_element)))

(fn AttachtoCachedCharacter
  (Transformation|AttachComponentToComponent (Variables|Default|GetMesh1P) (Variables|/Game/Connectia/Core/Characters/BP_ConnectiaCharacter.BP_ConnectiaCharacter_C|GetMesh1P (Variables|Default|GetCachedCharacter)) "KludgeWeaponSocket" "KeepRelative" "KeepRelative" "KeepRelative" true)
  (Transformation|AttachComponentToComponent (Variables|Default|GetMesh3P) (Variables|/Script/Engine.Character|GetMesh (Variables|Default|GetCachedCharacter)) "WeaponSocket" "KeepRelative" "KeepRelative" "KeepRelative" true))

(fn CacheOwnerCharacter
  (bind _asbp_connectia_character (Utilities|Casting|CastToBP_ConnectiaCharacter (Components|GetOwner)))
  (Variables|Default|SetCachedCharacter _asbp_connectia_character))