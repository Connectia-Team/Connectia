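; BP_DeathCamera is a camera actor that follows a target character's body, by its name for death views.
; On BeginPlay it attaches to the SpringEndpoint socket of the character's DeathCameraBoom.
; Each tick it smoothly interpolates that boom toward the mesh's spine_05 socket with VInterpTo, so the view tracks the body.
; It destroys itself once the target character is no longer valid.
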(event EventTick
  (params (DeltaSeconds :type Float%20%28single-precision%29))
  (bind _targetcharacter (Variables|Default|GetTargetCharacter))
  (bind _deathcameraboom (Variables|/Game/Connectia/Characters/BP_ConnectiaCharacter.BP_ConnectiaCharacter_C|GetDeathCameraBoom _targetcharacter))
  (Utilities|IsValid _targetcharacter
    (:Is%20Valid
      (Transformation|SetWorldLocation _deathcameraboom (Math|Interpolation|VInterpTo (Transformation|GetWorldLocation _deathcameraboom) (Transformation|GetSocketLocation (Variables|/Script/Engine.Character|GetMesh _targetcharacter) "spine_05") (Utilities|Time|GetWorldDeltaSeconds) 2e+01) false false))
    (:Is%20Not%20Valid
      (Actor|DestroyActor))))

(event EventBeginPlay
  (Transformation|AttachComponentToComponent (Variables|/Game/Connectia/Characters/BP_ConnectiaCharacter.BP_ConnectiaCharacter_C|GetDeathCameraBoom (Variables|Default|GetTargetCharacter)) "SpringEndpoint" "KeepRelative" "KeepRelative" "KeepRelative" true))

(fn ConstructionScript)