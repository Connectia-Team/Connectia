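; Leveling component that tracks player XP, level and stats, and pushes changes to the XP and stats widgets.
; AddXP fills the bar below max level and hands overflow to IncreaseLevel, which raises the capped XP requirement and recursively re-adds the remainder.
; Level-ups from level 1 onward grant skill points, which UpdateStats spends on HP, damage or magazine capacity.
; CurrentXP's RepNotify broadcasts OnXPChanged, while the Stats RepNotify is empty.
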(fn AddXP
  (params (Amount :type Float%20%28double-precision%29))
  (LocalVariables|SetlocalAddedXP (+ (Variables|Default|GetCurrentXP) Amount))
  (Variables|Default|SetOldXPPercentage (/ (Variables|Default|GetCurrentXP) (Variables|Default|GetMaxXP)))
  (if (< (Variables|Default|GetCurrentLevel) (Variables|Default|GetMaxLevel))
    (if (> (LocalVariables|GetlocalAddedXP) (Variables|Default|GetMaxXP))
      (LocalVariables|SetlocalGivenXP (- (Variables|Default|GetMaxXP) (Variables|Default|GetCurrentXP)))
      (LocalVariables|SetlocalExtraXP (- (LocalVariables|GetlocalAddedXP) (Variables|Default|GetMaxXP)))
      (Variables|Default|SetCurrentXP (+ (Variables|Default|GetCurrentXP) (LocalVariables|GetlocalGivenXP)))
      (else
        (Variables|Default|SetCurrentXP (LocalVariables|GetlocalAddedXP))))
    (Development|PrintString (Utilities|String|ToString(Text) (Utilities|Text|FormatText "{Current}/{Max}" (* (Variables|Default|GetCurrentXP) 1e+02) (* (Variables|Default|GetMaxXP) 1e+02))))
    (Default|UpdateXP (Variables|Default|GetPlayerXPWidgetReference))
    (LocalVariables|SetlocalGivenXP 0.0)
    (CallFunction|IncreaseLevel (LocalVariables|GetlocalExtraXP))))

(fn IncreaseLevel
  (params (ExtraXP :type Float%20%28double-precision%29))
  (bind _playerxpwidgetreference (Variables|Default|GetPlayerXPWidgetReference))
  (bind _stats (Variables|Default|GetStats))
  (bind _playerstatswidgetreference (Variables|Default|GetPlayerStatsWidgetReference))
  (bind _returnvalue (+ (.skillpoints _stats) 1))
  (bind _border (Variables|/Game/Connectia/UI/LevelingSystem/WBP_Stats.WBP_Stats_C|GetBorder _playerstatswidgetreference))
  (if (>= (Variables|Default|GetCurrentXP) (Variables|Default|GetMaxXP))
    (if (< (Variables|Default|GetCurrentLevel) 1)
      _
      (else
        (Utilities|Struct|SetmembersinPlayer_Stats_Structure (Variables|Default|GetStats) _returnvalue)
        (Rendering|Components|TextRender|SetText (Variables|/Game/Connectia/UI/LevelingSystem/WBP_Stats.WBP_Stats_C|GetSkillPoints _playerstatswidgetreference) (Utilities|Text|ToText(Integer) _returnvalue))
        (if (Widget|IsVisible _border)
          _
          (else
            (Widget|SetVisibility _border "Visible")
            (Variables|/Script/UMG.TextBlock|SetText (Variables|/Game/Connectia/UI/LevelingSystem/WBP_Stats.WBP_Stats_C|GetShowHideText _playerstatswidgetreference) "hide")))))
    (Variables|Default|SetCurrentLevel (+ (Variables|Default|GetCurrentLevel) 1))
    (Variables|Default|SetCurrentXP 0.0)
    (Variables|Default|SetMaxXP (Math|Float|Clamp(Float) (+ (Variables|Default|GetMaxXP) 0.5) 0.0 1e+01))
    (Default|UpdateLevel _playerxpwidgetreference)
    (Default|UpdateXP _playerxpwidgetreference)
    (if (> ExtraXP 0.0)
      (CallFunction|AddXP ExtraXP))))

(fn UpdateStats
  (params (StatName :type String))
  (bind _stats (Variables|Default|GetStats))
  (bind _stats_2 (Variables|Default|GetStats))
  (bind _returnvalue (+ (.hp _stats_2) 20))
  (bind _returnvalue_2 (- (.skillpoints _stats_2) 1))
  (bind _returnvalue_3 (+ (.damage _stats_2) 4))
  (bind _returnvalue_4 (+ (.magazinecap _stats_2) 6))
  (switch string StatName
    (:HP
      (Utilities|FlowControl|Sequence
        (:then_0
          (Utilities|Struct|SetmembersinPlayer_Stats_Structure _stats _returnvalue _returnvalue_2))
        (:then_1
          (return _returnvalue_2 _returnvalue))))
    (:Damage
      (Utilities|FlowControl|Sequence
        (:then_0
          (Utilities|Struct|SetmembersinPlayer_Stats_Structure _stats _returnvalue_3 _returnvalue_2))
        (:then_1
          (return _returnvalue_2 _returnvalue_3))))
    (:MagazineCap
      (Utilities|FlowControl|Sequence
        (:then_0
          (Utilities|Struct|SetmembersinPlayer_Stats_Structure _stats _returnvalue_4 _returnvalue_2))
        (:then_1
          (return _returnvalue_2 _returnvalue_4))))))

(fn OnRepStats)

(fn OnRepCurrentXP
  (Default|CallOnXPChanged self))

(fn Test
  (Variables|Default|SetCurrentXP (+ (Variables|Default|GetCurrentXP) 1e+01)))