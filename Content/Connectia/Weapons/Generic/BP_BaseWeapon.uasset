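; Base hitscan weapon for Connectia characters, with first and third person meshes, auto or single fire, magazine ammo and reloading.
; The owning client traces shots immediately and sends them to the server, which validates them, applies falloff-scaled damage and replicates LastShot for other clients to replay.
; Local recoil samples normal distributions from stability curves and gradually feeds into control rotation on a timer.
; Debug console variables expose server traces and unregistered client hits.
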(event Custom|Server_Reload
  (Variables|Default|SetIsReloading true)
  (if (not (Pawn|IsLocallyControlled (Variables|Default|GetOwnerCharacter)))
    (CallFunction|StartReloadInternal)))

(event Custom|Server_Shot
  (params (ShotData :type S%20Shot%20Data%20Structure) (DebugLastShotHitFromClient :type BP%20Connectia%20Character%20Object%20Reference))
  (Variables|Debug|UnregisteredHits|SetDebugLastShotHitFromClient DebugLastShotHitFromClient)
  (Utilities|AnticheatEnsure (CallFunction|CanMakeShot) (Utilities|Text|FormatText "Shooting when unable. MagazineAmmo={MagazineAmmo}. IsReloading={IsReloading}" (CallFunction|GetMagazineAmmo) (Variables|Default|GetIsReloading))
    (:Valid
      (bind _output_get (Variables|Default|SetLastShot ShotData))
      (if (not (Pawn|IsLocallyControlled (Variables|Default|GetOwnerCharacter)))
        (CallFunction|ShotInternal (.origin _output_get) (.direction _output_get))))))

(event EventBeginPlay
  (CallFunction|CacheOwnerCharacter :!label _label)
  (Utilities|IsValid (Variables|Default|GetOwnerCharacter)
    (:Is%20Valid
      (Variables|Default|SetIsInitialized true)
      (Utilities|FlowControl|Sequence
        (:then_0
          (CallFunction|AttachtoOwnerCharacter))
        (:then_1
          (if (Pawn|IsLocallyControlled (Variables|Default|GetOwnerCharacter))
            (bind _asplayer_controller (Utilities|Casting|CastToPlayerController (Pawn|GetController (Variables|Default|GetOwnerCharacter))))
            (Input|EnableInput _asplayer_controller)
            (EventDispatchers|AssignOnPrimaryActionPressed (Variables|Default|GetOwnerCharacter) (EventDispatchers|CreateEvent :!event StartShooting))
            (EventDispatchers|AssignOnPrimaryActionReleased (Variables|Default|GetOwnerCharacter) (EventDispatchers|CreateEvent :!event StopShooting))))
        (:then_2
          (Networking|SwitchHasAuthority
            (:Authority
              (CallFunction|SetMagazineAmmo (Variables|StaticConfigData|GetStaticMagazineCapacity)))))))
    (:Is%20Not%20Valid
      (Utilities|FlowControl|DelayUntilNextTick)
      (goto _label))))

(event Input|ActionEvents|InputActionReload
  (params (Key :type Key%20Structure))
  (:Pressed
    (CallFunction|Reload)))

(event Input|MouseEvents|DebugKeyMouseWheelUp
  (params (Key :type Key%20Structure) (ActionValue :type Input%20Action%20Value%20Structure))
  (bind _staticstability (Variables|StaticConfigData|GetStaticStability))
  (:Pressed
    (|SetBy-RefVar _staticstability (+ _staticstability 0.1))
    (Development|PrintString (Utilities|String|Append "New stability: " (Utilities|String|ToString(Float) (Variables|StaticConfigData|GetStaticStability))) true true "(R=1.000000,G=0.871763,B=0.000000,A=1.000000)" 2.0 "SetDebugStability")))

(event Input|MouseEvents|DebugKeyMouseWheelDown
  (params (Key :type Key%20Structure) (ActionValue :type Input%20Action%20Value%20Structure))
  (bind _staticstability (Variables|StaticConfigData|GetStaticStability))
  (:Pressed
    (|SetBy-RefVar _staticstability (- _staticstability 0.1))
    (Development|PrintString (Utilities|String|Append "New stability: " (Utilities|String|ToString(Float) (Variables|StaticConfigData|GetStaticStability))) true true "(R=1.000000,G=0.871763,B=0.000000,A=1.000000)" 2.0 "SetDebugStability")))

(fn ConstructionScript
  (for _array_element (Actor|GetComponentsByClass "/Script/Engine.MeshComponent")
    (CallFunction|MakeMeshAllMaterialsDynamic _array_element)))

(fn AttachtoOwnerCharacter
  (Transformation|AttachComponentToComponent (Variables|Default|GetMesh1P) (Variables|/Game/Connectia/Characters/BP_ConnectiaCharacter.BP_ConnectiaCharacter_C|GetMesh1P (Variables|Default|GetOwnerCharacter)) "KludgeWeaponSocket" "KeepRelative" "KeepRelative" "KeepRelative" true)
  (Transformation|AttachComponentToComponent (Variables|Default|GetMesh3P) (Variables|/Script/Engine.Character|GetMesh (Variables|Default|GetOwnerCharacter)) "WeaponSocket" "KeepRelative" "KeepRelative" "KeepRelative" true))

(fn CacheOwnerCharacter
  (bind _asbp_connectia_character (Utilities|Casting|CastToBP_ConnectiaCharacter (Components|GetOwner)))
  (Variables|Default|SetOwnerCharacter _asbp_connectia_character))

(fn StartShooting
  (if (not (Variables|Default|GetIsInShootingCooldown))
    (Variables|Default|SetWantsToShoot true)
    (CallFunction|TryMakeShot)))

(fn StopShooting
  (Variables|Default|SetWantsToShoot false))

(fn CanMakeShot
  (return (and (> (CallFunction|GetMagazineAmmo) 0) (not (Variables|Default|GetIsReloading)))))

(fn TryMakeShot
  (if (CallFunction|CanMakeShot)
    (Variables|Default|SetIsInShootingCooldown true)
    (Utilities|Time|SetTimerbyFunctionName 0 "OnShotCooldownElapsed" (Variables|StaticConfigData|GetStaticFireRateSecondsPerRound))
    (CallFunction|MakeShot)
    (else
      (Variables|Default|SetWantsToShoot false))))

(fn OnShotCooldownElapsed
  (Variables|Default|SetIsInShootingCooldown false)
  (if (Variables|Default|GetWantsToShoot)
    (switch Utilities|FlowControl|Switch|SwitchonE_FireMode (Variables|StaticConfigData|GetFireMode)
      (:NewEnumerator0
        (CallFunction|TryMakeShot))
      (:NewEnumerator1
        (CallFunction|StopShooting)
        (Variables|Default|SetWantsToShoot false)))))

(fn MakeShot
  (bind _ownercharacter (Variables|Default|GetOwnerCharacter))
  (bind _returnvalue (Pawn|GetController _ownercharacter))
  (bind (_location _rotation) (Pawn|GetPlayerViewPoint _returnvalue))
  (LocalVariables|SetOrigin _location)
  (LocalVariables|SetDirection (Math|Random|RandomUnitVectorinConeinDegrees (Math|Vector|GetForwardVector _rotation) (Variables|StaticConfigData|GetSpreadHalfAngleInDegrees)))
  (CallFunction|ShotInternal (LocalVariables|GetOrigin) (LocalVariables|GetDirection))
  (CallFunction|ServerShot (Utilities|Struct|MakeS_ShotData (LocalVariables|GetOrigin) (Math|Vector|MakeVectorNetQuantizeNormal (.x (LocalVariables|GetDirection)) (.y (LocalVariables|GetDirection)) (.z (LocalVariables|GetDirection))) (Math|Random|RandomIntegerinRange 1 (Utilities|MaxInteger))) (Variables|Debug|UnregisteredHits|GetDebugLastShotHit)))

(fn ShotInternal
  (params (Origin :type Vector) (Direction :type Vector))
  (bind _staticstability (Variables|StaticConfigData|GetStaticStability))
  (bind _debuglastshothitfromclient (Variables|Debug|UnregisteredHits|GetDebugLastShotHitFromClient))
  (bind _recoilprops (CallFunction|GetRecoilProps _staticstability))
  (bind _returnvalue (Development|GetConsoleVariableBoolValue "Connectia.Shooting.ServerDebugTraces"))
  (bind (_outhit _returnvalue_2) (Collision|LineTraceByChannel Origin (+ Origin (* Direction (Variables|StaticConfigData|GetStaticRange))) "TraceTypeQuery3" false (Utilities|Array|MakeArray (Variables|Default|GetOwnerCharacter)) (select (and (Ability|HasAuthority) _returnvalue) "ForDuration" "None")))
  (Utilities|FlowControl|Sequence
    (:then_0
      ;[1 1 1] Spawn and activate Weapon Decal System
      (Networking|CanExecuteCosmeticEvents
        (:True
          (if _returnvalue_2
            (Utilities|IsValid (Variables|Default|GetWeaponDecals)
              (:Is%20Valid
                _)
              (:Is%20Not%20Valid
                (bind _returnvalue_3 (Game|SpawnActorfromClass "/Game/Effects/Blueprints/B_WeaponDecals.B_WeaponDecals_C" (Math|Transform|MakeTransform "0, 0, 0") "Undefined" 0 0))
                (bind _output_get (Variables|Default|SetWeaponDecals _returnvalue_3))
                (Transformation|AttachComponentToComponent _output_get (Variables|Default|GetDefaultSceneRoot) "None" "KeepRelative" "KeepRelative" "KeepRelative" true)))
            (Variables|/Game/Effects/Blueprints/B_WeaponDecals.B_WeaponDecals_C|SetImpactPositions (Variables|Default|GetWeaponDecals) (Utilities|Array|MakeArray (.impactpoint _outhit)))
            (Variables|/Game/Effects/Blueprints/B_WeaponDecals.B_WeaponDecals_C|SetImpactNormals (Variables|Default|GetWeaponDecals) (Utilities|Array|MakeArray (.impactnormal _outhit)))
            (Variables|/Game/Effects/Blueprints/B_WeaponDecals.B_WeaponDecals_C|SetImpact%20Surface%20Types (Variables|Default|GetWeaponDecals) (Utilities|Array|MakeArray "SurfaceType2"))
            (Default|Fire (Variables|Default|GetWeaponDecals))))))
    (:then_1
      ;[1 1 1] Deal damage
      (Networking|SwitchHasAuthority
        (:Authority
          (if _returnvalue_2
            (bind _asbp_connectia_character (Utilities|Casting|CastToBP_ConnectiaCharacter (.hitactor _outhit)))
            (Game|Damage|ApplyDamage _asbp_connectia_character (* (Variables|StaticConfigData|GetStaticDamage) (Math|Curves|GetFloatValue (Variables|StaticConfigData|GetDamageFalloffCurve) (/ (.distance _outhit) (Variables|StaticConfigData|GetStaticRange)))) 0 0 "/Game/Connectia/DamageTypes/BP_InstantDamageType.BP_InstantDamageType_C")))))
    (:then_2
      ;[1 1 1] Debug unregistered hits
      (bind _asbp_connectia_character_2 (Utilities|Casting|CastToBP_ConnectiaCharacter (.hitactor _outhit))
        (:then
          _)
        (:CastFailed
          _))
      (Variables|Debug|UnregisteredHits|SetDebugLastShotHit _asbp_connectia_character_2)
      (Networking|SwitchHasAuthority
        (:Authority
          (if (not (Pawn|IsLocallyControlled (Variables|Default|GetOwnerCharacter)))
            (Utilities|IsValid _debuglastshothitfromclient
              (:Is%20Valid
                (if (not (or (Variables|/Game/Connectia/Characters/BP_ConnectiaCharacter.BP_ConnectiaCharacter_C|GetIsAlreadyDead _debuglastshothitfromclient) (== (Variables|Debug|UnregisteredHits|GetDebugLastShotHit) (Variables|Debug|UnregisteredHits|GetDebugLastShotHitFromClient))))
                  (bind _returnvalue_4 (Development|GetConsoleVariableBoolValue "Connectia.Shooting.UnregisteredHitsInfo"))
                  (if _returnvalue_4
                    (Development|PrintText (Utilities|Text|FormatText "The hit from the client {Client} was not registered" (Pawn|GetController (Variables|Default|GetOwnerCharacter))) true true "(R=1.000000,G=0.000000,B=0.000000,A=1.000000)")))))))))
    (:then_3
      ;[1 1 1] Fire montage
      (CallFunction|PlayMontage1P3P (Variables|Animations|Weapon|GetWeaponFireMontage) (Variables|Animations|Weapon|GetWeaponFireMontage))
      (Default|PlayMontage1P3P (Variables|Default|GetOwnerCharacter) (Variables|Animations|Character|GetCharacter1PFireMontage) (Variables|Animations|Character|GetCharacter3PFireMontage)))
    (:then_4
      ;[1 1 1] Update ammo
      (CallFunction|SetMagazineAmmo (- (CallFunction|GetMagazineAmmo) 1)))
    (:then_5
      ;[1 1 1] Add pending recoil
      (if (Pawn|IsLocallyControlled (Variables|Default|GetOwnerCharacter))
        (CallFunction|AddPendingRecoilYawPitchOffset (CallFunction|SampleNormalDistribution (.yawmean _recoilprops) (.yawstd _recoilprops)) (CallFunction|SampleNormalDistribution (.pitchmean _recoilprops) (.pitchstd _recoilprops)))))))

(fn OnRepLastShot
  (bind _lastshot (Variables|Default|GetLastShot))
  (if (Variables|Default|GetIsInitialized) ; TODO: Maybe it can be done better
    (Networking|SwitchHasAuthority
      (:Remote
        (CallFunction|ShotInternal (.origin _lastshot) (.direction _lastshot))))))

(fn SetMagazineAmmo
  (params (MagazineAmmo :type Integer))
  (Variables|Default|SetMagazineAmmo MagazineAmmo)
  (Default|CallOnAmmoChanged self))

(fn GetMagazineAmmo
  (return (Variables|Default|GetMagazineAmmo)))

(fn PlayMontage1P3P
  (params (1PMontage :type Anim%20Montage%20Object%20Reference) (3PMontage :type Anim%20Montage%20Object%20Reference))
  (if (Default|Isin1P (Variables|Default|GetOwnerCharacter))
    (bind _returnvalue (Animation|Montage|MontagePlay (Components|SkeletalMesh|GetAnimInstance (Variables|Default|GetMesh1P)) 1PMontage 1.0 "MontageLength" 0.0 true))
    (return _returnvalue)
    (else
      (bind _returnvalue_2 (Animation|Montage|MontagePlay (Components|SkeletalMesh|GetAnimInstance (Variables|Default|GetMesh3P)) 3PMontage 1.0 "MontageLength" 0.0 true))
      (return _returnvalue_2))))

(fn StopMontage1P3P
  (params (1PMontage :type Anim%20Montage%20Object%20Reference) (3PMontage :type Anim%20Montage%20Object%20Reference))
  (if (Default|Isin1P (Variables|Default|GetOwnerCharacter))
    (Animation|Montage|MontageStop (Components|SkeletalMesh|GetAnimInstance (Variables|Default|GetMesh1P)) 0.0 1PMontage)
    (else
      (Animation|Montage|MontageStop (Components|SkeletalMesh|GetAnimInstance (Variables|Default|GetMesh3P)) 0.0 3PMontage))))

(fn CanReload
  (return (not (Variables|Default|GetIsReloading))))

(fn Reload
  (if (CallFunction|CanReload)
    (Variables|Default|SetWantsToShoot false)
    (CallFunction|ServerReload)
    (CallFunction|StartReloadInternal)
    (Networking|SwitchHasAuthority
      (:Remote
        (Variables|Default|SetIsReloading true)))))

(fn OnRepIsReloading
  (if (Variables|Default|GetIsInitialized)
    (if (not (or (Ability|HasAuthority) (Pawn|IsLocallyControlled (Variables|Default|GetOwnerCharacter))))
      (if (Variables|Default|GetIsReloading)
        (CallFunction|StartReloadInternal)
        (else
          (CallFunction|StopReloadInternal))))))

(fn StartReloadInternal
  (Default|PlayMontage1P3P (Variables|Default|GetOwnerCharacter) (Variables|Animations|Character|GetCharacter1PReloadMontage) (Variables|Animations|Character|GetCharacter3PReloadMontage)))

(fn StopReloadInternal
  (Default|StopMontage1P3P (Variables|Default|GetOwnerCharacter) (Variables|Animations|Character|GetCharacter1PReloadMontage) (Variables|Animations|Character|GetCharacter3PReloadMontage)))

(fn OnReloadedInternal
  (if (or (Ability|HasAuthority) (Pawn|IsLocallyControlled (Variables|Default|GetOwnerCharacter)))
    (Variables|Default|SetIsReloading false)
    (Networking|SwitchHasAuthority
      (:Authority
        (CallFunction|SetMagazineAmmo (Variables|StaticConfigData|GetStaticMagazineCapacity))))))

(fn OnRepMagazineAmmo
  (if (Variables|Default|GetIsInitialized)
    (Networking|SwitchHasAuthority
      (:Remote
        (Default|CallOnAmmoChanged self)))))

(fn GetRecoilProps
  (params (Stability :type Float%20%28double-precision%29))
  (bind _yawpitchmeancurve (Variables|StaticConfigData|Recoil|GetYawPitchMeanCurve))
  (bind _yawpitchstdcurve (Variables|StaticConfigData|Recoil|GetYawPitchStdCurve))
  (bind _returnvalue (Math|Curves|GetVectorValue _yawpitchmeancurve Stability))
  (bind _returnvalue_2 (Math|Curves|GetVectorValue _yawpitchstdcurve Stability))
  (return (Utilities|Struct|MakeS_RecoilProperties (.x _returnvalue) (.x _returnvalue_2) (.y _returnvalue) (.y _returnvalue_2))))

(fn AddPendingRecoilYawPitchOffset
  (params (DeltaYaw :type Float%20%28double-precision%29) (DeltaPitch :type Float%20%28double-precision%29))
  (bind _output_get (Variables|Default|SetPendingRecoilYawPitchOffset (+ (Variables|Default|GetPendingRecoilYawPitchOffset) (Math|Vector2D|MakeVector2D DeltaYaw DeltaPitch))))
  (if (and (not (Class|KismetMathLibrary|IsNearlyZero2D _output_get 0.0001)) (not (Utilities|Time|IsTimerActivebyHandle (Variables|Default|GetAbsorbPartOfRecoilTimerHandle))))
    (bind _returnvalue (Utilities|Time|SetTimerbyFunctionName 0 "OnAbsorbPartOfRecoilTimerElapsed" (Variables|Default|GetAbsorbPartOfRecoilTimerDelay) true))
    (Variables|Default|SetAbsorbPartOfRecoilTimerHandle _returnvalue)))

(fn OnAbsorbPartOfRecoilTimerElapsed
  (bind _isfullyabsorbed (CallFunction|ControllerAbsorbPartOfRecoil (Variables|Default|GetAbsorbPartOfRecoilTimerDelay)))
  (if _isfullyabsorbed
    (Utilities|Time|ClearandInvalidateTimerbyHandle (Variables|Default|GetAbsorbPartOfRecoilTimerHandle))))

(fn ControllerAbsorbPartOfRecoil
  (params (DeltaSeconds :type Float%20%28double-precision%29))
  (bind _ownercharacter (Variables|Default|GetOwnerCharacter))
  (bind _returnvalue (Pawn|GetController _ownercharacter))
  (bind _returnvalue_2 (Pawn|GetControlRotation _returnvalue :!class /Script/Engine.Controller))
  (if (Pawn|IsLocallyControlled _ownercharacter)
    (bind _output_get (LocalVariables|SetNewPendingRecoilYawPitchOffset (Math|Conversions|ToVector2D(Vector) (Math|Interpolation|VInterpTo (Math|Conversions|ToVector(Vector2D) (Variables|Default|GetPendingRecoilYawPitchOffset)) "0, 0, 0" DeltaSeconds (Variables|Default|GetRecoilAbsorbtionSpeed)))))
    (Pawn|SetControlRotation _returnvalue (Math|Rotator|MakeRotator (.roll _returnvalue_2) (+ (.pitch _returnvalue_2) (.y (- (Variables|Default|GetPendingRecoilYawPitchOffset) _output_get))) (+ (.yaw _returnvalue_2) (.x (- (Variables|Default|GetPendingRecoilYawPitchOffset) _output_get)))))
    (bind _output_get_2 (Variables|Default|SetPendingRecoilYawPitchOffset (LocalVariables|GetNewPendingRecoilYawPitchOffset)))
    (return (Class|KismetMathLibrary|IsNearlyZero2D _output_get_2 0.0001))
    (else
      (return false))))

(fn GetActualMesh
  (if (Default|Isin1P (Variables|Default|GetOwnerCharacter))
    (return (Variables|Default|GetMesh1P))
    (else
      (return (Variables|Default|GetMesh3P)))))